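; Player-drivable SUV pawn built on Chaos wheeled vehicle movement.
; Input events feed throttle, brake, steering and handbrake to the movement component, and turn and look input rotate the controller.
; While steering, Tick steps a clamped SteeringAngle by one, its direction inferred by comparing the first two wheels' absolute steer angles.
; With zero steering input, the MoveRight axis event eases that angle back to zero.
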(event EventTick
  (params (DeltaSeconds :type Float%20%28single-precision%29))
  (if (Variables|Default|GetisSteering)
    (bind _newparam (CallFunction|SteeringWheelUpdate))
    (if (== _newparam 1.0)
      (Variables|Default|SetSteeringAngle (Math|Float|Clamp(Float) (+ (Variables|Default|GetSteeringAngle) _newparam) (Variables|Default|GetSteeringAngle) (Variables|Default|GetMaxSteeringWheel)))
      (else
        (Variables|Default|SetSteeringAngle (Math|Float|Clamp(Float) (+ (Variables|Default|GetSteeringAngle) _newparam) (Variables|Default|GetMinSteeringWheel) (Variables|Default|GetSteeringAngle)))))))

(event EventBeginPlay
  (bind _aschaos_wheeled_vehicle_movement_component (Utilities|Casting|CastToChaosWheeledVehicleMovementComponent (Variables|Default|GetVehicleMovementComponent)))
  (Variables|Default|SetAs%20Chaos%20Wheeled%20Vehicle%20Movement%20Component _aschaos_wheeled_vehicle_movement_component))

(event Input|ActionEvents|InputActionHandbrake
  (params (Key :type Key%20Structure :default "None"))
  (bind _vehiclemovementcomponent (Variables|Default|GetVehicleMovementComponent))
  (:Pressed
    (Class|ChaosVehicleMovementComponent|SetHandbrakeInput _vehiclemovementcomponent true)
    (Variables|Default|SetIs%20Handbrake%20on? true))
  (:Released
    (Class|ChaosVehicleMovementComponent|SetHandbrakeInput _vehiclemovementcomponent false)
    (Variables|Default|SetIs%20Handbrake%20on? false)))

(event Input|AxisEvents|InputAxisMoveRight
  (params (AxisValue :type Float%20%28single-precision%29))
  (Class|ChaosVehicleMovementComponent|SetSteeringInput (Variables|Default|GetVehicleMovementComponent) AxisValue)
  (if (== AxisValue 0.0)
    (Variables|Default|SetisSteering false)
    (if (> (Variables|Default|GetSteeringAngle) 0.0)
      (Variables|Default|SetSteeringAngle (Math|Float|Clamp(Float) (- (Variables|Default|GetSteeringAngle) 1.0) 0.0 (Variables|Default|GetSteeringAngle)))
      (elif (not (== (Variables|Default|GetSteeringAngle) 0.0))
        (Variables|Default|SetSteeringAngle (Math|Float|Clamp(Float) (+ (Variables|Default|GetSteeringAngle) 1.0) (Variables|Default|GetSteeringAngle) 0.0))))
    (else
      (Variables|Default|SetisSteering true))))

(event Input|AxisEvents|InputAxisTurn
  (params (AxisValue :type Float%20%28single-precision%29))
  (Pawn|Input|AddControllerYawInput AxisValue))

(event Input|AxisEvents|InputAxisLookUp
  (params (AxisValue :type Float%20%28single-precision%29))
  (Pawn|Input|AddControllerPitchInput AxisValue))

(event Input|AxisEvents|InputAxisMoveForward
  (params (AxisValue :type Float%20%28single-precision%29))
  (Class|ChaosVehicleMovementComponent|SetThrottleInput (Variables|Default|GetVehicleMovementComponent) AxisValue))

(event Input|AxisEvents|InputAxisReverse/Brake
  (params (AxisValue :type Float%20%28single-precision%29))
  (Class|ChaosVehicleMovementComponent|SetBrakeInput (Variables|Default|GetVehicleMovementComponent) AxisValue))

(fn ConstructionScript)

(fn SteeringWheelUpdate
  (bind _as_chaos_wheeled_vehicle_movement_component (Variables|Default|GetAs%20Chaos%20Wheeled%20Vehicle%20Movement%20Component))
  (bind _wheels (Variables|/Script/ChaosVehicles.ChaosWheeledVehicleMovementComponent|GetWheels _as_chaos_wheeled_vehicle_movement_component))
  (if (> (Math|Float|Absolute(Float) (Class|ChaosVehicleWheel|GetSteerAngle (Utilities|Array|Get(acopy) _wheels))) (Math|Float|Absolute(Float) (Class|ChaosVehicleWheel|GetSteerAngle (Utilities|Array|Get(acopy) _wheels 1))))
    (return -1.0)
    (else
      (return 1.0))))